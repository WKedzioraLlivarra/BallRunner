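; Player-controlled rolling ball actor that moves by physics torque and restarts the level when it takes damage.
; Forward/back and left/right axis inputs apply acceleration-based torque to the sphere, scaled by a force multiplier.
; Any damage triggers, once, a camera fade, then after a short delay reloads the current level by name.
; A ChangeCamerView function sets spring arm length and rotation.
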(event `InputAxis|ForwadBack`
  (params (AxisValue :type "Float (single-precision)"))
  ;[1 1 1] ball _movement
  (`PrimitiveComponent.AddTorqueInRadians` (`self.Sphere`) (`KismetMathLibrary.MakeVector` 0.0 (* AxisValue (`self.Force Multiplay`))) "None" true))

(event `InputAxis|LeftRight`
  (params (AxisValue :type "Float (single-precision)"))
  ;[1 1 1] ball _movement
  (`PrimitiveComponent.AddTorqueInRadians` (`self.Sphere`) (`KismetMathLibrary.MakeVector` (* AxisValue (`self.Force Multiplay`))) "None" true))

(event `self.ReceiveAnyDamage`
  (params (Damage :type "Float (single-precision)") (DamageType :type "DamageType Object Reference") (InstigatedBy :type "Controller Object Reference") (DamageCauser :type "Actor Object Reference"))
  ;[1 0.5034 0.5833] Death
  (`/Engine/EditorBlueprintResources/StandardMacros.DoOnce` false
    (:`Completed`
      (`PlayerCameraManager.StartCameraFade` :`self` (`GameplayStatics.GetPlayerCameraManager` 0) :`Duration` 1.0 :`bHoldWhenFinished` true)
      (`KismetSystemLibrary.Delay` 1.0)
      (bind _returnvalue (`GameplayStatics.GetCurrentLevelName` true))
      (`GameplayStatics.OpenLevel` (`KismetStringLibrary.Conv_StringToName` _returnvalue)))))

(fn `changeCamerView`
  (params (CameraPosition :type "Float (double-precision)") (CameraRotationY :type "Float (double-precision)") (CameraRotationZ :type "Float (double-precision)"))
  (bind _springarm (`self.SpringArm`))
  (set `SpringArmComponent.TargetArmLength` CameraPosition _springarm)
  (`SceneComponent.K2_SetWorldRotation` _springarm (`KismetMathLibrary.MakeRotator` 0.0 CameraRotationY CameraRotationZ) false false))

(fn `UserConstructionScript`)