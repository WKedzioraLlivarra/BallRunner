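; BP_Spikes_01 is a spike hazard that damages the player pawn.
; Damage is applied when the first player's pawn ends overlap with component R, rather than on entering it.
; An unwired timeline chain would slide the Cone along relative X and call Play again after a short delay.
; BeginPlay is empty, so that movement never runs.
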(event `self.r.OnComponentEndOverlap`
  (params (OverlappedComponent :type "PrimitiveComponent Object Reference") (OtherActor :type "Actor Object Reference") (OtherComp :type "PrimitiveComponent Object Reference") (OtherBodyIndex :type Integer))
  ;[1 0.04093 0.1807] Death
  (if (== OtherActor (`GameplayStatics.GetPlayerPawn` 0))
    (`GameplayStatics.ApplyDamage` OtherActor 1.0)))

(event `self.ReceiveBeginPlay`
  ;[0.2746 0.612 1] Spike Movment
)

(fn `UserConstructionScript`)