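; BP_Canon is a cannon actor that fires BP_projectile automatically and continuously from BeginPlay.
; After a short delay it spawns a scaled-down projectile at the Arrow component's location and rotation.
; The Canon_fire timeline then slides the Cannon component along relative Y, and its Finished output restarts the cycle.
; The separate SpawnProjectile function is empty, with a disconnected spawn node left unused.
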(event `self.ReceiveBeginPlay`
  (bind _arrow (`self.Arrow`))
  (`KismetSystemLibrary.Delay` 0.2 :!label _label)
  (`|SpawnActorFromClass` "/Game/BP_actors/BP_projectile/BP_projectile.BP_projectile_C" (`KismetMathLibrary.MakeTransform` (`SceneComponent.K2_GetComponentLocation` _arrow) (`SceneComponent.K2_GetComponentRotation` _arrow) (0.25 0.25 0.25)) "Undefined" "OverrideRootScale" null null)
  (bind (_direction _canon_fire) (`Timeline|Canon_fire` :`NewTime` (`self.Duration`) :!via `PlayFromStart`)
    (:`Update`
      (`SceneComponent.K2_SetRelativeLocation` (`self.Cannon`) (`KismetMathLibrary.MakeVector` 0.0 _canon_fire) false false))
    (:`Finished`
      (goto _label))))

(fn `Spawn Projectile`)

(fn `UserConstructionScript`)